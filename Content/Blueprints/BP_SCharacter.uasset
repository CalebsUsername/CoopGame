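; BP_SCharacter is a character Blueprint that handles the aim-down-sights camera offset and the local player's HUD.
; Every tick it snaps the CameraBoom socket offset between two fixed positions based on IsADSight, with no interpolation.
; On BeginPlay, only for the locally controlled instance, it creates the crosshair and health bar widgets and adds them to the viewport.
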(event `self.ReceiveTick`
  (params (DeltaSeconds :type "Float (single-precision)"))
  (`|ExecutionSequence`
    (:`then_0`
      (if (`self.bIsADSight`)
        (set `SpringArmComponent.SocketOffset` (0.0 10.0 15.0) (`self.CameraBoom`))
        (else
          (set `SpringArmComponent.SocketOffset` (0.0 15.0 10.0) (`self.CameraBoom`)))))))

(event `self.ReceiveBeginPlay`
  (if (`self.IsLocallyControlled`)
    (`|ExecutionSequence`
      (:`then_0`
        (bind _returnvalue (`|CreateWidget` "/Game/UI/WBP_Crosshair.WBP_Crosshair_C"))
        (`UserWidget.AddToViewport` _returnvalue 0))
      (:`then_1`
        (bind _returnvalue_2 (`|CreateWidget` "/Game/UI/WBP_HealthBar.WBP_HealthBar_C"))
        (`UserWidget.AddToViewport` _returnvalue_2 0)))))

(fn `UserConstructionScript`)