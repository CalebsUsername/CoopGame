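; Super Speed power-up that doubles the walk speed of the player who activates it until it expires.
; OnActivated stores the player and sets MaxWalkSpeed to twice GetMaxSpeed(), while OnExpired sets it to half the current GetMaxSpeed() and calls the parent expiry.
; Both pass the new speed to ReplicatesMovementMaxWalkSpeed, which reapplies it to that player's CharacterMovementComponent.
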(event `self.OnActivated`
  (params (ActivateFor :type "Actor Object Reference"))
  (bind _returnvalue (`self.GetComponentByClass` ActivateFor "/Script/Engine.CharacterMovementComponent"))
  (set `self.ActivatedForPlayer` ActivateFor)
  (`/Engine/EditorBlueprintResources/StandardMacros.IsValid` _returnvalue
    (:`Is Valid`
      (bind _output_get (set `CharacterMovementComponent.MaxWalkSpeed` (* (`MovementComponent.GetMaxSpeed` _returnvalue) 2.0) _returnvalue))
      (`self.Replicates MovementMaxWalkSpeed` _output_get (`self.ActivatedForPlayer`)))))

(event `self.OnExpired`
  (bind _returnvalue (`self.GetComponentByClass` (`self.ActivatedForPlayer`) "/Script/Engine.CharacterMovementComponent"))
  (`/Engine/EditorBlueprintResources/StandardMacros.IsValid` _returnvalue
    (:`Is Valid`
      (bind _output_get (set `CharacterMovementComponent.MaxWalkSpeed` (/ (`MovementComponent.GetMaxSpeed` _returnvalue) 2.0) _returnvalue))
      (`self.Replicates MovementMaxWalkSpeed` _output_get (`self.ActivatedForPlayer`))
      (`parent.OnExpired`))
    (:`Is Not Valid`
      (`parent.OnExpired`))))

(event `Replicates MovementMaxWalkSpeed`
  (params (NewMaxWalkSpeed :type "Float (double-precision)") (OwningActor :type "Actor Object Reference"))
  (set `CharacterMovementComponent.MaxWalkSpeed` NewMaxWalkSpeed (`self.GetComponentByClass` OwningActor "/Script/Engine.CharacterMovementComponent")))

(fn `UserConstructionScript`)