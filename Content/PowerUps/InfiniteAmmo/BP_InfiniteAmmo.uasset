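; Infinite ammo power-up that keeps the affected BP_SCharacter's current weapon magazine topped up while it runs.
; Each power-up tick sets the valid current weapon's magazine size to a fixed high value rather than disabling ammo consumption.
; On expiry, it resets whichever weapon is then current to its base magazine size, and the parent expiry logic runs in every case.
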(event `self.OnPowerUpTicked`
  (bind _asbp_scharacter (cast `/Game/Blueprints/BP_SCharacter` (stale `self.OnActivated` ActivateFor)))
  (bind _currentweapon (`SCharacter.CurrentWeapon` _asbp_scharacter))
  (`/Engine/EditorBlueprintResources/StandardMacros.IsValid` _currentweapon
    (:`Is Valid`
      (set `SWeapon.CurrentMagSize` 100.0 _currentweapon))))

(event `self.OnActivated`
  (params (ActivateFor :type "Actor Object Reference")))

(event `self.OnExpired`
  (bind _asbp_scharacter (cast `/Game/Blueprints/BP_SCharacter` (stale `self.OnActivated` ActivateFor))
    (:`then`
      (bind _currentweapon (`SCharacter.CurrentWeapon` _asbp_scharacter))
      (`/Engine/EditorBlueprintResources/StandardMacros.IsValid` _currentweapon
        (:`Is Valid`
          (set `SWeapon.CurrentMagSize` (`SWeapon.BaseMagazineSize` _currentweapon) _currentweapon)
          (`parent.OnExpired`))
        (:`Is Not Valid`
          (`parent.OnExpired` :!label _label))))
    (:`CastFailed`
      (goto _label))))

(fn `OnRep_Activate For`)

(fn `UserConstructionScript`
  (`parent.UserConstructionScript`))