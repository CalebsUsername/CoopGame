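; Behavior tree task that heals the AI-controlled pawn through its SHealthComponent.
; It restores 15% of DefaultHealth at once, then makes two further Heal calls with a zero amount at one-second intervals.
; The task finishes successfully after about three seconds, or calls FinishAbort if the pawn has no health component.
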(event `self.ReceiveExecuteAI`
  (params (OwnerController :type "AIController Object Reference") (ControlledPawn :type "Pawn Object Reference"))
  (bind _returnvalue (`Actor.GetComponentByClass` ControlledPawn "/Script/CoopGame.SHealthComponent"))
  (`/Engine/EditorBlueprintResources/StandardMacros.IsValid` _returnvalue
    (:`Is Valid`
      (bind _output_get (set `self.Amount` (* (`SHealthComponent.DefaultHealth` _returnvalue) 0.15)))
      (`SHealthComponent.Heal` _returnvalue _output_get)
      (`KismetSystemLibrary.Delay` 1.0)
      (`SHealthComponent.Heal` _returnvalue 0.0)
      (`KismetSystemLibrary.Delay` 1.0)
      (`SHealthComponent.Heal` _returnvalue 0.0)
      (`KismetSystemLibrary.Delay` 1.0)
      (`self.FinishExecute` true))
    (:`Is Not Valid`
      (`self.FinishAbort`))))